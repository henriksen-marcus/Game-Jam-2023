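; BP_Podium is a Capture the Flag scoring podium that awards a team point when a flag carrier reaches it.
; On BeginPlay it binds its capsule's begin-overlap event, which checks for a BP_FirstPersonCharacter carrying a flag and clears that carrying state.
; It then tells the CTF_GMB game mode to raise the Blue or Red score based on the podium's BlueTeam flag, without checking the carrier's team.
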(event Custom|OnComponentBeginOverlap_Event
  (params (OverlappedComponent :type Primitive%20Component%20Object%20Reference) (OtherActor :type Actor%20Object%20Reference) (OtherComp :type Primitive%20Component%20Object%20Reference) (OtherBodyIndex :type Integer) (bFromSweep :type Boolean) (SweepResult :type Hit%20Result%20Structure%20%28by%20ref%29))
  (bind _asbp_first_person_character (Utilities|Casting|CastToBP_FirstPersonCharacter OtherActor))
  (if (Variables|/Game/FirstPerson/Blueprints/BP_FirstPersonCharacter.BP_FirstPersonCharacter_C|GetcarryingFlag _asbp_first_person_character)
    (Default|ToggleCarryingFlag _asbp_first_person_character false)
    (bind _asctf_gmb (Utilities|Casting|CastToCTF_GMB (Game|GetGameMode)))
    (if (Variables|Default|GetBlueTeam)
      (Default|IncreaseScoreBlue _asctf_gmb)
      (else
        (Default|IncreaseScoreRed _asctf_gmb)))))

(event EventBeginPlay
  (Collision|AssignOnComponentBeginOverlap (Variables|Default|GetCapsule) (delegate Custom|OnComponentBeginOverlap_Event)))

(fn ConstructionScript)