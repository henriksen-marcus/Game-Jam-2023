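; Capture-the-flag base flag for one team that handles stealing and scoring through capsule overlaps with first-person characters.
; While the flag is home, an enemy touch gives that player the flag, hides the mesh and notifies CTF_GMB that it left base.
; A teammate touching it while carrying a flag increases their team's score in the game mode.
; ResetFlag restores visibility and the held state.
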(event Custom|OnComponentBeginOverlap_Event
  (params (OverlappedComponent :type Primitive%20Component%20Object%20Reference) (OtherActor :type Actor%20Object%20Reference) (OtherComp :type Primitive%20Component%20Object%20Reference) (OtherBodyIndex :type Integer) (bFromSweep :type Boolean) (SweepResult :type Hit%20Result%20Structure%20%28by%20ref%29))
  (bind _returnvalue (Game|GetGameMode))
  (if (Variables|Default|GetisHoldingFlag)
    (bind _asbp_first_person_character (Utilities|Casting|CastToBP_FirstPersonCharacter OtherActor))
    (bind _isenemyteam (CallFunction|IsEnemyTeam _asbp_first_person_character))
    (if _isenemyteam
      (Default|ToggleCarryingFlag _asbp_first_person_character true)
      (bind _asctf_gmb (Utilities|Casting|CastToCTF_GMB _returnvalue))
      (if (Variables|Default|GetisBlueTeam)
        (Default|IsFlaginBaseBlue _asctf_gmb false)
        (else
          (Default|IsFlaginBaseRed _asctf_gmb false)))
      (Rendering|SetVisibility (Variables|Default|GetFlagMesh) false false)
      (Variables|Default|SetisHoldingFlag false)
      (elif (Variables|/Game/FirstPerson/Blueprints/BP_FirstPersonCharacter.BP_FirstPersonCharacter_C|GetcarryingFlag _asbp_first_person_character)
        (bind _asctf_gmb_2 (Utilities|Casting|CastToCTF_GMB _returnvalue))
        (if (Variables|/Game/FirstPerson/Blueprints/BP_FirstPersonCharacter.BP_FirstPersonCharacter_C|GetisBlueTeam _asbp_first_person_character)
          (Default|IncreaseScoreBlue _asctf_gmb_2)
          (Development|PrintString "INCRS SCOR BLUE")
          (else
            (Default|IncreaseScoreRed _asctf_gmb_2)
            (Development|PrintString "IUNRS SCOR RED")))))))

(event EventBeginPlay
  (Collision|AssignOnComponentBeginOverlap (Variables|Default|GetCapsuleCollision) (delegate Custom|OnComponentBeginOverlap_Event)))

(fn ConstructionScript)

(fn IsEnemyTeam
  (params (Player :type BP%20First%20Person%20Character%20Object%20Reference))
  (if (== (Variables|/Game/FirstPerson/Blueprints/BP_FirstPersonCharacter.BP_FirstPersonCharacter_C|GetisBlueTeam Player) (Variables|Default|GetisBlueTeam))
    (return false)
    (else
      (return true))))

(fn ResetFlag
  (Rendering|SetVisibility (Variables|Default|GetFlagMesh) true false)
  (Variables|Default|SetisHoldingFlag true))